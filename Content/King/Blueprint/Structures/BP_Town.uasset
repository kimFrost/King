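; BP_Town is a town structure that periodically sends out convoys loaded with resources from its surrounding tiles.
; Gather spawns a BP_Convoy with the town as source, then loads Lumber for each adjacent Forest tile, otherwise Wheat if fertile.
; ReturnConvoy, called on BeginPlay, sets a one-shot timer for Gather, so further cycles depend on it being called again from outside this Blueprint.
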(event `self.ReceiveBeginPlay`
  (`parent.ReceiveBeginPlay`)
  (`self.ReturnConvoy`))

(event `self.ReceiveTick`
  (params (DeltaSeconds :type "Float (single-precision)"))
  (`parent.ReceiveTick` DeltaSeconds))

(fn `Gather`
  (`/Engine/EditorBlueprintResources/StandardMacros.IsValid` (`self.TileOn`)
    (:`Is Valid`
      (bind _convoy (`self.SpawnConvoy`))
      (`/Engine/EditorBlueprintResources/StandardMacros.IsValid` _convoy
        (:`Is Valid`
          (for _array_element (`/Game/King/Blueprint/Tiles/BP_Tile.AdjacentTiles` (`self.TileOn`))
            (`/Engine/EditorBlueprintResources/StandardMacros.IsValid` _array_element
              (:`Is Valid`
                (if (`KismetArrayLibrary.Array_Contains` (`/Game/King/Blueprint/Tiles/BP_Tile.TileLayers` _array_element) "Forest")
                  (`/Game/King/Blueprint/BP_Convoy.LoadResource` _convoy "Lumber")
                  (elif (`/Game/King/Blueprint/Tiles/BP_Tile.IsFertile` _array_element)
                    (`/Game/King/Blueprint/BP_Convoy.LoadResource` _convoy "Wheat")))))))))))

(fn `ReturnConvoy`
  (`KismetSystemLibrary.K2_SetTimer` null "Gather" 5.0))

(fn `SpawnConvoy`
  (returns (Convoy :type "/Game/King/Blueprint/BP_Convoy Object Reference"))
  (bind _returnvalue (`|SpawnActorFromClass` :`Class` "/Game/King/Blueprint/BP_Convoy.BP_Convoy_C" :`SpawnTransform` (`KismetMathLibrary.Conv_VectorToTransform` (`self.K2_GetActorLocation`)) :`CollisionHandlingOverride` "AlwaysSpawn" :`TransformScaleMethod` "OverrideRootScale" :`TownSource` self :`Instigator` null))
  (return _returnvalue))

(fn `UserConstructionScript`
  (`parent.UserConstructionScript`))
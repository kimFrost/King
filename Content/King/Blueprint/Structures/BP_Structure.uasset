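; Base structure actor that sits on a map tile, with stub Construct and AddLabour functions.
; On BeginPlay it traces down to find its BP_Tile, reruns Construct on that tile's stat updates, and adds stat provider components from its Data.
; If pathing is enabled, a looping timer clears its destination info on all road layers, then rebroadcasts itself as a destination through adjacent tiles' roads.
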(event `self.ReceiveBeginPlay`
  (bind _returnvalue (`self.K2_GetActorLocation`))
  (`|ExecutionSequence`
    (:`then_0`
      (bind (_outhit _returnvalue_2) (`KismetSystemLibrary.LineTraceSingle` (+ _returnvalue (0.0 0.0 100.0)) (+ _returnvalue (0.0 0.0 -100.0)) "TraceTypeQuery3"))
      (if _returnvalue_2
        (bind _asbp_tile (cast `/Game/King/Blueprint/Tiles/BP_Tile` (`.HitActor` (`GameplayStatics.BreakHitResult` _outhit))))
        (bind _output_get (set `self.TileOn` _asbp_tile))
        (add `/Game/King/Blueprint/Tiles/BP_Tile.OnTileStatsUpdate` _output_get (delegate `_OnTileStatsUpdate`))
        (for _array_element (`.StatProviders` (break `ST_Structure` (`self.Data`)))
          (`AddComponent|NODE_AddStatProviderComponent-1` :`Data` _array_element))))
    (:`then_1`
      (if (`.bIncludePathing` (break `ST_Structure` (`self.Data`)))
        (`KismetSystemLibrary.K2_SetTimerDelegate` (delegate `CustomEvent_0`) 5.0 true)
        (`self.UpdatePathing`)))))

(event `_OnTileStatsUpdate`
  (`self.Update`))

(event `CustomEvent_0`
  (`self.UpdatePathing`))

(fn `AddLabour`
  (returns (LabourAdded :type Boolean))
  (return false))

(fn `AddResource`
  (params (ID :type String) (Amount :type "Float (double-precision)"))
  (`self.ResourceAdded` ID Amount))

(fn `Construct`)

(fn `Update`
  (`self.Construct`))

(fn `UpdatePathing`
  (bind _tileon (`self.TileOn`))
  (`|ExecutionSequence`
    (:`then_0`
      (bind _outactors (`GameplayStatics.GetAllActorsOfClass` "/Game/King/Blueprint/Tiles/Layers/BP_TileLayer_Road.BP_TileLayer_Road_C"))
      (for _array_element _outactors
        (`/Engine/EditorBlueprintResources/StandardMacros.IsValid` _array_element
          (:`Is Valid`
            (`/Game/King/Blueprint/Tiles/Layers/BP_TileLayer_Road.ClearDestinationInfo` _array_element self)))))
    (:`then_1`
      (`/Engine/EditorBlueprintResources/StandardMacros.IsValid` _tileon
        (:`Is Valid`
          (for _array_element_2 (`/Game/King/Blueprint/Tiles/BP_Tile.AdjacentTiles` _tileon)
            (`/Engine/EditorBlueprintResources/StandardMacros.IsValid` _array_element_2
              (:`Is Valid`
                (bind _road (`/Game/King/Blueprint/Tiles/BP_Tile.GetRoad` _array_element_2))
                (`/Engine/EditorBlueprintResources/StandardMacros.IsValid` _road
                  (:`Is Valid`
                    (`/Game/King/Blueprint/Tiles/Layers/BP_TileLayer_Road.BroadcastDestination` _road self 1)))))))))))

(fn `UserConstructionScript`
  (`self.Construct`))
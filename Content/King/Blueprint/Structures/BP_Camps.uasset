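; BP_Camps is a camp structure that spreads Safety to the tile grid and tracks its own safety need.
; Each tick it pushes time-scaled Safety from its tile at distance 1 and draws the need value as debug text.
; Resource-added events raise the need value by the received amount, without checking the resource ID.
; When the need hits zero, both instanced static mesh components are scaled down to flattened shapes.
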(event `self.ReceiveBeginPlay`
  (`parent.ReceiveBeginPlay`)
  (add `self.ResourceAdded` (delegate `CustomEvent_0`)))

(event `CustomEvent_0` :!signature `self.ResourceAdded`
  (params (ID :type String) (Amount :type "Float (double-precision)"))
  (bind _safetyneedcomponent (`self.SafetyNeedComponent`))
  (set `/Game/King/Blueprint/Components/NeedComponent.Value` (+ (`/Game/King/Blueprint/Components/NeedComponent.Value` _safetyneedcomponent) Amount) _safetyneedcomponent))

(event `self.ReceiveTick`
  (params (DeltaSeconds :type "Float (single-precision)"))
  (bind _tileon (`self.TileOn`))
  (`parent.ReceiveTick` DeltaSeconds)
  (`KismetSystemLibrary.DrawDebugString` (`self.K2_GetActorLocation`) (`KismetStringLibrary.Conv_DoubleToString` (`/Game/King/Blueprint/Components/NeedComponent.Value` (`self.SafetyNeedComponent`))))
  (`/Engine/EditorBlueprintResources/StandardMacros.IsValid` _tileon
    (:`Is Valid`
      (`/Game/King/Blueprint/Tiles/BP_Tile.PushResource` _tileon "Safety" DeltaSeconds 1))))

(event `self.SafetyNeedComponent.OnNeedZero`
  (`SceneComponent.SetWorldScale3D` (`self.InstancedStaticMesh`) (0.5 0.5 0.01))
  (`SceneComponent.SetWorldScale3D` (`self.InstancedStaticMesh1`) (0.5 0.5 0.01)))

(fn `UserConstructionScript`
  (`parent.UserConstructionScript`))
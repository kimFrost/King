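; BP_Neighbour is a prototype actor that shows a Widget_Neighbour and holds an array of neighbours to match by In and Out values.
; BeginPlay adds the widget component and caches a reference to its widget.
; A custom event shuffles the neighbours and compares each valid one's In to this actor's Out, but nothing follows the check.
; The random delay and looping timer meant to drive that event are disconnected, so they never run.
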(event `self.ReceiveBeginPlay`
  (`|ExecutionSequence`
    (:`then_0`
      (bind _returnvalue (`AddComponent|NODE_AddWidgetComponent-0`))
      (bind _output_get (set `self.WidgetComponent` _returnvalue))
      (bind _aswidget_neighbour (cast `/Game/King/Blueprint/UI/Widgets/Widget_Neighbour` (`WidgetComponent.GetUserWidgetObject` _output_get)))
      (set `self.WidgetRef` _aswidget_neighbour))))

(event `CustomEvent_0`
  (bind _neighbours (`self.Neighbours`))
  (`KismetArrayLibrary.Array_Shuffle` _neighbours)
  (for _array_element _neighbours
    (`/Engine/EditorBlueprintResources/StandardMacros.IsValid` _array_element
      (:`Is Valid`
        (if (`KismetStringLibrary.EqualEqual_StrStr` (`/Game/King/Blueprint/Structures/BP_Neighbour.In` _array_element) (`self.Out`))
          _)))))

(fn `UserConstructionScript`)
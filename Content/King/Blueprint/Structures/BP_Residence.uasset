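; BP_Residence is a settlement tile building that supplies the castle, sends out labourers and grows over time.
; It sends a convoy to the first BP_TestCastle on BeginPlay and periodically spawns a labourer toward a random adjacent tile.
; ReturnConvoy schedules Gather, which loads a new convoy from neighbouring forest and fertile tiles, then calls Grow to randomly densify or spread to a free neighbour.
; Instanced meshes draw Density-based scattered houses and fences on hex edges without roads or towns.
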(event `self.ReceiveBeginPlay`
  (`parent.ReceiveBeginPlay`)
  (`self.SpawnConvoy`)
  (`KismetSystemLibrary.K2_SetTimerDelegate` (delegate `CustomEvent_0`) 7.0 true))

(event `CustomEvent_0`
  (`self.SpawnLabourer`))

(event `self.ReceiveTick`
  (params (DeltaSeconds :type "Float (single-precision)"))
  (`parent.ReceiveTick` DeltaSeconds))

(event `self.Update`
  (`parent.Update`))

(event `self.Construct`
  (`parent.Construct`)
  (`self.PlantHouses`)
  (`self.ConstructFence`))

(fn `ConstructFence`
  (bind _tileon (`self.TileOn`))
  (`InstancedStaticMeshComponent.ClearInstances` (`self.FenceMeshes`))
  (`/Engine/EditorBlueprintResources/StandardMacros.IsValid` _tileon
    (:`Is Valid`
      (for (_array_element _array_index) (`/Game/King/Blueprint/Tiles/BP_Tile.AdjacentTiles` _tileon)
        (`/Engine/EditorBlueprintResources/StandardMacros.IsValid` _array_element
          (:`Is Valid`
            (bind _hasit (`/Game/King/Blueprint/Tiles/BP_Tile.HasThis` _array_element (`|MakeArray`) (`|MakeArray` "Road" "Town")))
            (if _hasit
              (`InstancedStaticMeshComponent.AddInstance` (`self.FenceMeshes`) (`KismetMathLibrary.MakeTransform` (0.0 0.0 0.0) (`KismetMathLibrary.MakeRotator` 0.0 0.0 (* _array_index 60.0)))))))))))

(fn `EmitLabour`
  (locals (_AdjacentTiles :type "Array of /Game/King/Blueprint/Tiles/BP_Tile Object Reference"))
  (bind _tileon (`self.TileOn`))
  (bind __adjacenttiles (`local._AdjacentTiles`))
  (`/Engine/EditorBlueprintResources/StandardMacros.IsValid` _tileon
    (:`Is Valid`
      (bind _output_get (set `local._AdjacentTiles` (`/Game/King/Blueprint/Tiles/BP_Tile.AdjacentTiles` _tileon)))
      (for _array_element _output_get
        (`/Engine/EditorBlueprintResources/StandardMacros.IsValid` _array_element))
      (`KismetArrayLibrary.Array_Shuffle` __adjacenttiles)
      (for _array_element_2 __adjacenttiles
        (`/Engine/EditorBlueprintResources/StandardMacros.IsValid` _array_element_2
          (:`Is Valid`
            (bind _isfree (`/Game/King/Blueprint/Tiles/BP_Tile.IsFree` _array_element_2))
            (if _isfree
              (bind _labouradded (`/Game/King/Blueprint/Tiles/BP_Tile.AddLabour` _array_element_2))
              (if _labouradded
                (return)))))))
    (:`Is Not Valid`
      (return))))

(fn `Gather`
  (`/Engine/EditorBlueprintResources/StandardMacros.IsValid` (`self.TileOn`)
    (:`Is Valid`
      (bind _convoy (`self.SpawnConvoy`))
      (`/Engine/EditorBlueprintResources/StandardMacros.IsValid` _convoy
        (:`Is Valid`
          (for _array_element (`/Game/King/Blueprint/Tiles/BP_Tile.AdjacentTiles` (`self.TileOn`))
            (`/Engine/EditorBlueprintResources/StandardMacros.IsValid` _array_element
              (:`Is Valid`
                (if (`KismetArrayLibrary.Array_Contains` (`/Game/King/Blueprint/Tiles/BP_Tile.TileLayers` _array_element) "Forest")
                  (`/Game/King/Blueprint/BP_Convoy.LoadResource` _convoy "Lumber")
                  (elif (`/Game/King/Blueprint/Tiles/BP_Tile.IsFertile` _array_element)
                    (`/Game/King/Blueprint/BP_Convoy.LoadResource` _convoy "Wheat")))))))))))

(fn `Grow`
  (locals (_AdjacentTiles :type "Array of /Game/King/Blueprint/Tiles/BP_Tile Object Reference"))
  (bind _tileon (`self.TileOn`))
  (`/Engine/EditorBlueprintResources/StandardMacros.IsValid` _tileon
    (:`Is Valid`
      (if (`KismetMathLibrary.RandomBool`)
        (`/Engine/EditorBlueprintResources/StandardMacros.IncrementInt` (`self.Density`)
          (:`  `
            (`self.PlantHouses`)
            (return)))
        (else
          (bind _output_get (set `local._AdjacentTiles` (`/Game/King/Blueprint/Tiles/BP_Tile.AdjacentTiles` _tileon)))
          (`KismetArrayLibrary.Array_Shuffle` _output_get)
          (for _array_element _output_get
            (`/Engine/EditorBlueprintResources/StandardMacros.IsValid` _array_element
              (:`Is Valid`
                (bind _isfree (`/Game/King/Blueprint/Tiles/BP_Tile.IsFree` _array_element))
                (if _isfree
                  (`|SpawnActorFromClass` "BP_Residence_C" (`KismetMathLibrary.Conv_VectorToTransform` (`self.K2_GetActorLocation` _array_element)) "AlwaysSpawn" "OverrideRootScale" null 1 _array_element (`self.Data`) null)
                  (return)))))
          (return))))))

(fn `PlantHouses`
  (`InstancedStaticMeshComponent.ClearInstances` (`self.InstancedStaticMesh`))
  (for _ (range (`self.Density`))
    (`InstancedStaticMeshComponent.AddInstanceWorldSpace` (`self.InstancedStaticMesh`) (`KismetMathLibrary.MakeTransform` (`KismetMathLibrary.RandomPointInBoundingBox` (`self.K2_GetActorLocation`) (`KismetMathLibrary.MakeVector` 100.0 100.0)) (`KismetMathLibrary.MakeRotator` 0.0 0.0 (`KismetMathLibrary.RandomFloatInRange` 0.0 360.0)) (0.2 0.2 0.2)))))

(fn `ReturnConvoy`
  (`KismetSystemLibrary.K2_SetTimer` null "Gather" 2.0)
  (`self.Grow`))

(fn `SpawnConvoy`
  (returns (Convoy :type "/Game/King/Blueprint/BP_Convoy Object Reference"))
  (bind _outactors (`GameplayStatics.GetAllActorsOfClass` "/Game/King/Blueprint/Structures/BP_TestCastle.BP_TestCastle_C"))
  (for _array_element _outactors
    (bind _returnvalue (`|SpawnActorFromClass` "/Game/King/Blueprint/BP_Convoy.BP_Convoy_C" (`KismetMathLibrary.Conv_VectorToTransform` (`self.K2_GetActorLocation`)) "AlwaysSpawn" "OverrideRootScale" null (`|MakeArray` "Wheat" "Lumber") self _array_element null))
    (return _returnvalue)))

(fn `SpawnLabourer`
  (locals (_AdjacentTiles :type "Array of /Game/King/Blueprint/Tiles/BP_Tile Object Reference"))
  (bind _tileon (`self.TileOn`))
  (`/Engine/EditorBlueprintResources/StandardMacros.IsValid` _tileon
    (:`Is Valid`
      (bind _output_get (set `local._AdjacentTiles` (`/Game/King/Blueprint/Tiles/BP_Tile.AdjacentTiles` _tileon)))
      (`KismetArrayLibrary.Array_Shuffle` _output_get)
      (for _array_element _output_get
        (`/Engine/EditorBlueprintResources/StandardMacros.IsValid` _array_element
          (:`Is Valid`
            (bind _returnvalue (`|SpawnActorFromClass` "/Game/King/Blueprint/Characters/Labourer/BP_Labourer.BP_Labourer_C" (`KismetMathLibrary.Conv_VectorToTransform` (+ (`self.K2_GetActorLocation`) (0.0 0.0 20.0))) "AlwaysSpawn" "OverrideRootScale" null self null))
            (`/Engine/EditorBlueprintResources/StandardMacros.IsValid` _returnvalue
              (:`Is Valid`
                (`/Game/King/Blueprint/Characters/Labourer/BP_Labourer.GoToTile` _returnvalue _array_element)
                (return)))))))))

(fn `UserConstructionScript`
  (`parent.UserConstructionScript`))
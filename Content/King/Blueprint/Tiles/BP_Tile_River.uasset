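; BP_Tile_River is a river tile Blueprint with an unfinished spline-based river built in its construction script.
; After the parent construction script runs, it adds one spline mesh component per RiverSpline point.
; The new meshes never receive start and end positions or tangents.
; Point placement calls are disconnected, and the spline location, tangent and InDirection/OutDirection reads are unused.
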(fn `UserConstructionScript`
  (`parent.UserConstructionScript`)
  (`|ExecutionSequence`
    (:`then_1`
      (for _index (range (`SplineComponent.GetNumberOfSplinePoints` (`self.RiverSpline`)))
        (`AddComponent|NODE_AddSplineMeshComponent-0`)))))
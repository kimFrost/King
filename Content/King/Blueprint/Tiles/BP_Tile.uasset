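; BP_Tile is a hex map tile that holds terrain layers, stats and the structure standing on it.
; Line traces find six neighbours via cube coordinates and re-check the structure every second.
; Update sums base and provider stats (deduplicated by source ID), sets the grass material's Fertile parameter and refreshes layer child actors.
; Helpers push resources to neighbouring structures, spread rivers and forests, add farm fields and spawn farms from a data table.
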(event `self.ReceiveBeginPlay`
  (`self.TraceForNeighbors`)
  (`KismetSystemLibrary.K2_SetTimerDelegate` (delegate `CustomEvent_0`) 1.0 true)
  (`self.TraceForStructure`)
  (`self.Update`))

(event `CustomEvent_0`
  (`self.TraceForStructure`))

(fn `AddLabour`
  (returns (LabourAdded :type Boolean))
  (bind _tilelayers (`self.TileLayers`))
  (if (and (`.ReturnValue` (`BlueprintMapLibrary.Map_Find` (`self.Stats`) "Fertile")) (`KismetMathLibrary.BooleanNOR` (`KismetArrayLibrary.Array_Contains` _tilelayers "Forest") (`KismetArrayLibrary.Array_Contains` _tilelayers "River")))
    (`self.AddLayer` "FarmField")
    (return true)
    (else
      (return false))))

(fn `AddLayer`
  (params (ID :type String))
  (`KismetArrayLibrary.Array_AddUnique` (`self.TileLayers`) ID)
  (`self.ConstructLayers`))

(fn `AddProvider`
  (params (Provider :type "/Game/King/Blueprint/Components/StatProviderComponent Object Reference"))
  (bind _sourceid (`/Game/King/Blueprint/Components/StatProviderComponent.GetSourceID` Provider))
  (`/Engine/EditorBlueprintResources/StandardMacros.IsValid` Provider
    (:`Is Valid`
      (if (`KismetArrayLibrary.Array_Contains` (`self.StatProvidersInRange`) Provider)
        _
        (elif (`KismetStringLibrary.NotEqual_StrStr` _sourceid)
          (if (not (`BlueprintMapLibrary.Map_Contains` (`self.ProvidersBySourceID`) _sourceid))
            (`KismetArrayLibrary.Array_Add` (`self.StatProvidersInRange`) Provider :!label _label)
            (`BlueprintMapLibrary.Map_Add` (`self.ProvidersBySourceID`) _sourceid Provider)
            (`self.Update`))
          (else
            (goto _label)))))))

(fn `AddRunningLayer`
  (params (ID :type String))
  (bind _adjacenttiles (`self.AdjacentTiles`))
  (bind _output (`|GetArrayItem` _adjacenttiles 3))
  (bind _output_2 (`|GetArrayItem` _adjacenttiles 2))
  (`self.AddLayer` ID)
  (switch `string` ID
    (:`River`
      (if (`KismetMathLibrary.RandomBool`)
        (`/Engine/EditorBlueprintResources/StandardMacros.IsValid` _output_2
          (:`Is Valid`
            (`self.AddRunningLayer` _output_2 ID)))
        (else
          (`/Engine/EditorBlueprintResources/StandardMacros.IsValid` _output
            (:`Is Valid`
              (`self.AddRunningLayer` _output ID))))))
    (:`Forest`
      (for _array_element (`self.AdjacentTiles`)
        (`/Engine/EditorBlueprintResources/StandardMacros.IsValid` _array_element
          (:`Is Valid`
            (`self.AddLayer` _array_element ID)))))))

(fn `AddStat`
  (params (ID :type String) (Amount :type Integer))
  (bind (_value _returnvalue) (`BlueprintMapLibrary.Map_Find` (`self.Stats`) ID))
  (if (`BlueprintMapLibrary.Map_Contains` (`self.Stats`) ID)
    (if _returnvalue
      (`BlueprintMapLibrary.Map_Add` (`self.Stats`) ID (+ _value Amount)))
    (else
      (`BlueprintMapLibrary.Map_Add` (`self.Stats`) ID Amount))))

(fn `AddStats`
  (params (Stats :type "Map of String to Integer"))
  (bind _keys (`BlueprintMapLibrary.Map_Keys` Stats))
  (for _array_element _keys
    (bind (_value _returnvalue) (`BlueprintMapLibrary.Map_Find` Stats _array_element))
    (if _returnvalue
      (`self.AddStat` _array_element _value))))

(fn `ConstructLayers`
  (for _array_element (`self.TileLayers`)
    (switch `string` _array_element
      (:`Forest`
        (bind _returnvalue (`AddComponent|NODE_AddChildActorComponent-7`))
        (bind _asbp_tile_layer (cast `/Game/King/Blueprint/Tiles/Layers/BP_TileLayer` (`ChildActorComponent.ChildActor` _returnvalue)))
        (`KismetArrayLibrary.Array_Add` (`self.TileLayerActors`) _asbp_tile_layer))
      (:`River`
        (bind _returnvalue_2 (`AddComponent|NODE_AddChildActorComponent-8`))
        (bind _asbp_tile_layer_2 (cast `/Game/King/Blueprint/Tiles/Layers/BP_TileLayer` (`ChildActorComponent.ChildActor` _returnvalue_2)))
        (`KismetArrayLibrary.Array_Add` (`self.TileLayerActors`) _asbp_tile_layer_2))
      (:`Road`
        (bind _returnvalue_3 (`AddComponent|NODE_AddChildActorComponent-9`))
        (bind _asbp_tile_layer_3 (cast `/Game/King/Blueprint/Tiles/Layers/BP_TileLayer` (`ChildActorComponent.ChildActor` _returnvalue_3)))
        (`KismetArrayLibrary.Array_Add` (`self.TileLayerActors`) _asbp_tile_layer_3))
      (:`FarmField`
        (bind _returnvalue_4 (`AddComponent|NODE_AddChildActorComponent-10`))
        (bind _asbp_tile_layer_4 (cast `/Game/King/Blueprint/Tiles/Layers/BP_TileLayer` (`ChildActorComponent.ChildActor` _returnvalue_4)))
        (`KismetArrayLibrary.Array_Add` (`self.TileLayerActors`) _asbp_tile_layer_4))
      (:`Rocks`
        (bind _returnvalue_5 (`AddComponent|NODE_AddChildActorComponent-11`))
        (bind _asbp_tile_layer_5 (cast `/Game/King/Blueprint/Tiles/Layers/BP_TileLayer` (`ChildActorComponent.ChildActor` _returnvalue_5)))
        (`KismetArrayLibrary.Array_Add` (`self.TileLayerActors`) _asbp_tile_layer_5))
      (:`Manor`
        (bind _returnvalue_6 (`AddComponent|NODE_AddChildActorComponent-12`))
        (bind _asbp_tile_layer_6 (cast `/Game/King/Blueprint/Tiles/Layers/BP_TileLayer` (`ChildActorComponent.ChildActor` _returnvalue_6)))
        (`KismetArrayLibrary.Array_Add` (`self.TileLayerActors`) _asbp_tile_layer_6)))))

(fn `GetRoad`
  (returns (Road :type "/Game/King/Blueprint/Tiles/Layers/BP_TileLayer_Road Object Reference"))
  (for _array_element (`self.TileLayerActors`)
    (`/Engine/EditorBlueprintResources/StandardMacros.IsValid` _array_element
      (:`Is Valid`
        (bind _asbp_tile_layer_road (cast `/Game/King/Blueprint/Tiles/Layers/BP_TileLayer_Road` _array_element))
        (return _asbp_tile_layer_road))
      (:`Is Not Valid`
        (return null))))
  (return null))

(fn `HasThis`
  (params (Has :type "Array of String (by ref)") (HasNot :type "Array of String (by ref)"))
  (returns (HasIt :type Boolean))
  (for _array_element Has
    (if (not (`KismetArrayLibrary.Array_Contains` (`self.TileLayers`) _array_element))
      (return false)))
  (for _array_element_2 HasNot
    (if (`KismetArrayLibrary.Array_Contains` (`self.TileLayers`) _array_element_2)
      (return false)))
  (return true))

(fn `Initiate`
  (`|ExecutionSequence`
    (:`then_2`
      (`self.ConstructLayers`))
    (:`then_3`
      (`self.TraceForNeighbors`))
    (:`then_4`
      (`self.Update`))))

(fn `IsFree`
  (returns (IsFree :type Boolean))
  (`/Engine/EditorBlueprintResources/StandardMacros.IsValid` (`self.StructureOnTIle`)
    (:`Is Valid`
      (return false))
    (:`Is Not Valid`
      (return (== (`KismetArrayLibrary.Array_Length` (`self.TileLayers`)) 0)))))

(fn `PushResource`
  (params (ID :type String) (Amount :type "Float (double-precision)") (Distance :type Integer))
  (for _array_element (`self.AdjacentTiles`)
    (`/Engine/EditorBlueprintResources/StandardMacros.IsValid` _array_element
      (:`Is Valid`
        (bind _structureontile (`/Game/King/Blueprint/Tiles/BP_Tile.StructureOnTIle` _array_element))
        (`/Engine/EditorBlueprintResources/StandardMacros.IsValid` _structureontile
          (:`Is Valid`
            (`/Game/King/Blueprint/Structures/BP_Structure.AddResource` _structureontile ID Amount)))))))

(fn `RemoveProvider`
  (params (Provider :type "/Game/King/Blueprint/Components/StatProviderComponent Object Reference")))

(fn `SpawnStructure`
  (params (StructureID :type String))
  (bind _returnvalue (`|GetDataTableRow` "/Game/King/Blueprint/Data/DATA_Structures.DATA_Structures" (`KismetStringLibrary.Conv_StringToName` StructureID))
    (:`then`
      (switch `string` StructureID
        (:`Farm`
          (`|SpawnActorFromClass` "/Game/King/Blueprint/Structures/BP_FarmField.BP_FarmField_C" (`KismetMathLibrary.Conv_VectorToTransform` (`self.K2_GetActorLocation`)) "Undefined" "OverrideRootScale" null null _returnvalue null))))))

(fn `TraceForNeighbors`
  (bind _adjacenttiles (`self.AdjacentTiles`))
  (bind _returnvalue (`KingTilesLibrary.LocationToCube` 255.0 294.0 (`self.K2_GetActorLocation`)))
  (for _index (range 6)
    (bind _returnvalue_2 (`KingTilesLibrary.DirectionToCube` _index))
    (bind _returnvalue_3 (`KingTilesLibrary.CubeToLocation` (+ _returnvalue_2 _returnvalue)))
    (bind (_outhit _returnvalue_4) (`KismetSystemLibrary.LineTraceSingle` (+ _returnvalue_3 (0.0 0.0 -500.0)) (+ _returnvalue_3 (0.0 0.0 500.0)) "TraceTypeQuery3"))
    (if _returnvalue_4
      (bind _asbp_tile (cast `/Game/King/Blueprint/Tiles/BP_Tile` (`.HitActor` (`GameplayStatics.BreakHitResult` _outhit)))
        (:`then`
          (`KismetArrayLibrary.Array_Set` _adjacenttiles _index _asbp_tile))
        (:`CastFailed`
          (`KismetArrayLibrary.Array_Set` _adjacenttiles _index :!label _label)))
      (else
        (goto _label)))))

(fn `TraceForStructure`
  (bind _returnvalue (`self.K2_GetActorLocation`))
  (bind (_outhit _returnvalue_2) (`KismetSystemLibrary.LineTraceSingle` (+ _returnvalue (0.0 0.0 500.0)) (+ _returnvalue (0.0 0.0 -500.0)) "TraceTypeQuery4"))
  (if _returnvalue_2
    (bind _asbp_structure (cast `/Game/King/Blueprint/Structures/BP_Structure` (`.HitActor` (`GameplayStatics.BreakHitResult` _outhit)))
      (:`then`
        (set `self.StructureOnTIle` _asbp_structure))
      (:`CastFailed`
        (set `self.StructureOnTIle` null :!label _label)))
    (else
      (goto _label))))

(fn `Update`
  (`|ExecutionSequence`
    (:`then_0`
      (set `self.Stats` (`self.BaseStats`))
      (for _array_element (`self.StatProvidersInRange`)
        (`/Engine/EditorBlueprintResources/StandardMacros.IsValid` _array_element
          (:`Is Valid`
            (`self.AddStats` (`/Game/King/Blueprint/Components/StatProviderComponent.GetStats` _array_element)))))
      (`self.OnTileStatsUpdate`))
    (:`then_1`
      (`MaterialInstanceDynamic.SetScalarParameterValue` (`self.GroundMaterialDynaimicInstance`) "Fertile" (`KismetMathLibrary.Conv_IntToDouble` (`BlueprintMapLibrary.Map_Find` (`self.Stats`) "Fertile"))))
    (:`then_2`
      (for _array_element_2 (`self.TileLayerActors`)
        (`/Engine/EditorBlueprintResources/StandardMacros.IsValid` _array_element_2
          (:`Is Valid`
            (`/Game/King/Blueprint/Tiles/Layers/BP_TileLayer.Update` _array_element_2)))))))

(fn `UserConstructionScript`
  (bind _staticmesh (`self.StaticMesh`))
  (bind _returnvalue (`PrimitiveComponent.CreateDynamicMaterialInstance` _staticmesh 0 "/Game/King/Materials/M_Grass.M_Grass"))
  (bind _output_get (set `self.GroundMaterialDynaimicInstance` _returnvalue))
  (`PrimitiveComponent.SetMaterial` _staticmesh 0 _output_get))
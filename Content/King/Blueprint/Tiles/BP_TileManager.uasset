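; BP_TileManager builds a hex tile map on BeginPlay and seeds it with terrain layers.
; It spawns BP_Tile actors row by row, offsetting alternate rows by half a hex width, and stores them in an array.
; After all tiles exist, each traces for its neighbors.
; It then adds a River running layer at a fixed tile index and Forest layers at randomly picked indices.
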(event `self.ReceiveBeginPlay`
  (bind _tiles (`self.Tiles`))
  (bind _output (`|GetArrayItem` (`self.Tiles`) 8))
  (bind _output_2 (`|GetArrayItem` _tiles (`KismetMathLibrary.RandomIntegerInRange` 0 (- (`KismetArrayLibrary.Array_Length` _tiles) 1))))
  (`|ExecutionSequence`
    (:`then_0`
      (for _index (range (`self.NumOfRows`))
        (for _index_2 (range (`self.NumOfColumns`))
          (bind _returnvalue (`|SpawnActorFromClass` :`Class` "/Game/King/Blueprint/Tiles/BP_Tile.BP_Tile_C" :`SpawnTransform` (`KismetMathLibrary.Conv_VectorToTransform` (`KismetMathLibrary.MakeVector` (+ (* _index_2 (`self.HexWidth`)) (* (mod (+ _index 0) 2) (/ (`self.HexWidth`) 2.0))) (* _index (* (`self.HexHeight`) 0.75)) (`KismetMathLibrary.RandomFloatInRange` 0.0))) :`CollisionHandlingOverride` "AlwaysSpawn" :`TransformScaleMethod` "OverrideRootScale" :`BaseStats` (`self.DevTileBaseStats`) :`Instigator` null))
          (`KismetArrayLibrary.Array_Add` (`self.Tiles`) _returnvalue))))
    (:`then_1`
      (for _array_element (`self.Tiles`)
        (`/Engine/EditorBlueprintResources/StandardMacros.IsValid` _array_element
          (:`Is Valid`
            (`/Game/King/Blueprint/Tiles/BP_Tile.TraceForNeighbors` _array_element)))))
    (:`then_2`
      (`/Engine/EditorBlueprintResources/StandardMacros.IsValid` _output
        (:`Is Valid`
          (`/Game/King/Blueprint/Tiles/BP_Tile.AddRunningLayer` _output "River"))))
    (:`then_3`
      (for _ (range 21)
        (`/Engine/EditorBlueprintResources/StandardMacros.IsValid` _output_2
          (:`Is Valid`
            (`/Game/King/Blueprint/Tiles/BP_Tile.AddRunningLayer` _output_2 "Forest")))))))

(fn `UserConstructionScript`)
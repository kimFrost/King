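; BP_TileLayer_Road is a tile layer that builds a road piece across a tile between an incoming and an outgoing direction.
; The construction script moves the first and third points of RoadSpline to half the location offset of DirectionIn and DirectionOut.
; It then adds a spline mesh component for each spline segment, matching local positions and tangents so the road bends along the curve.
; There is no active runtime logic.
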(fn `UserConstructionScript`
  (bind _roadspline (`self.RoadSpline`))
  (bind _roadspline_2 (`self.RoadSpline`))
  (bind _roadspline_3 (`self.RoadSpline`))
  (`parent.UserConstructionScript`)
  (`|ExecutionSequence`
    (:`then_0`
      (bind _returnvalue (`KingTilesLibrary.DirectionToLocation` (`self.DirectionIn`)))
      (bind _returnvalue_2 (`KingTilesLibrary.DirectionToLocation` (`self.DirectionOut`)))
      (`SplineComponent.SetLocationAtSplinePoint` _roadspline 0 (/ _returnvalue 2.0) "Local" true)
      (`SplineComponent.SetLocationAtSplinePoint` _roadspline 2 (/ _returnvalue_2 2.0) "Local" true))
    (:`then_1`
      (for _index (range (+ (- (`SplineComponent.GetNumberOfSplinePoints` (`self.RoadSpline`)) 2) 1))
        (bind _returnvalue_3 (`AddComponent|NODE_AddSplineMeshComponent-0` :`bManualAttachment` true))
        (bind _returnvalue_4 (+ _index 1))
        (`SplineMeshComponent.SetStartAndEnd` _returnvalue_3 (`SplineComponent.GetLocationAtSplinePoint` _roadspline_3 _index "Local") (`SplineComponent.GetTangentAtSplinePoint` _roadspline_3 _index "Local") (`SplineComponent.GetLocationAtSplinePoint` _roadspline_2 _returnvalue_4 "Local") (`SplineComponent.GetTangentAtSplinePoint` _roadspline_2 _returnvalue_4 "Local") true)
        (`SceneComponent.K2_AttachToComponent` _returnvalue_3 (`self.RoadSpline`) "None" "KeepRelative" "KeepRelative" "KeepRelative" true)))))
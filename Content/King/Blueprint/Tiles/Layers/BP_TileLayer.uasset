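; BP_TileLayer is an actor that sits on a map tile and records which BP_Tile it is on.
; On BeginPlay it line traces vertically through its location and stores the hit BP_Tile in TileOn, clearing it if the hit actor is not a tile.
; Update is an empty function, and the construction script only calls its parent.
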(event `self.ReceiveBeginPlay`
  (bind _returnvalue (`self.K2_GetActorLocation`))
  (bind (_outhit _returnvalue_2) (`KismetSystemLibrary.LineTraceSingle` (+ _returnvalue (0.0 0.0 100.0)) (+ _returnvalue (0.0 0.0 -100.0)) "TraceTypeQuery3"))
  (if _returnvalue_2
    (bind _asbp_tile (cast `/Game/King/Blueprint/Tiles/BP_Tile` (`.HitActor` (`GameplayStatics.BreakHitResult` _outhit)))
      (:`then`
        (set `self.TileOn` _asbp_tile))
      (:`CastFailed`
        (set `self.TileOn` null)))))

(fn `Update`)

(fn `UserConstructionScript`
  (`parent.UserConstructionScript`))
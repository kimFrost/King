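; Farm field tile layer that fills a tile with instanced field meshes and fences its borders.
; The construction script lays out centered rows from FieldRowLayout on a fixed spacing, with random roll and yaw per instance.
; On BeginPlay and Update, ConstructFence rebuilds fence instances in 60-degree hex steps, on sides whose valid neighbor tile lacks FarmField.
; Older square-layout and random-scatter placement logic remains unconnected.
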(event `self.ReceiveBeginPlay`
  (`parent.ReceiveBeginPlay`)
  (`self.ConstructFence` :!label _label))

(event `self.Update`
  (`parent.Update`)
  (goto _label))

(fn `ConstructFence`
  (bind _tileon (`self.TileOn`))
  (`InstancedStaticMeshComponent.ClearInstances` (`self.FenceMeshes`))
  (`/Engine/EditorBlueprintResources/StandardMacros.IsValid` _tileon
    (:`Is Valid`
      (for (_array_element _array_index) (`/Game/King/Blueprint/Tiles/BP_Tile.AdjacentTiles` _tileon)
        (`/Engine/EditorBlueprintResources/StandardMacros.IsValid` _array_element
          (:`Is Valid`
            (bind _hasit (`/Game/King/Blueprint/Tiles/BP_Tile.HasThis` _array_element (`|MakeArray`) (`|MakeArray` "FarmField")))
            (if _hasit
              (`InstancedStaticMeshComponent.AddInstance` (`self.FenceMeshes`) (`KismetMathLibrary.MakeTransform` (0.0 0.0 0.0) (`KismetMathLibrary.MakeRotator` 0.0 0.0 (* _array_index 60.0)))))))))))

(fn `UserConstructionScript`
  (bind _fieldrowlayout (`self.FieldRowLayout`))
  (`parent.UserConstructionScript`)
  (for (_array_element _array_index) _fieldrowlayout
    (bind _returnvalue (- _array_element 1))
    (for _index (range (+ _returnvalue 1))
      (`InstancedStaticMeshComponent.AddInstance` (`self.Meshes`) (`KismetMathLibrary.MakeTransform` (`KismetMathLibrary.MakeVector` (- (* _index 10.0) (* (* _returnvalue 0.5) 10.0)) (- (* _array_index 10.0) (* 10.0 (* (`KismetArrayLibrary.Array_Length` _fieldrowlayout) 0.5)))) (`KismetMathLibrary.MakeRotator` (`KismetMathLibrary.RandomFloatInRange` -40.0 -20.0) 0.0 (`KismetMathLibrary.RandomFloatInRange` -10.0 10.0)))))))
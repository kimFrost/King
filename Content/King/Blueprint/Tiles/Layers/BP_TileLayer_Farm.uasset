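; Farm tile layer that scatters about 500 mesh instances over a flat square centered on the actor.
; After the parent construction script, a loop adds each instance to Meshes at a random world-space point, re-randomized whenever construction runs.
; A downward-trace branch that checks for a BP_Tile hit is present but disconnected, so placement does no ground or tile check.
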(fn `UserConstructionScript`
  (`parent.UserConstructionScript`)
  (for _ (range 501)
    (`InstancedStaticMeshComponent.AddInstanceWorldSpace` (`self.Meshes`) (`KismetMathLibrary.Conv_VectorToTransform` (`KismetMathLibrary.RandomPointInBoundingBox` (`self.K2_GetActorLocation`) (`KismetMathLibrary.MakeVector` 100.0 100.0))))))
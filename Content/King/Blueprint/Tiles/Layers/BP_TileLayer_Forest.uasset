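; Forest tile layer that scatters tree meshes over the tile beneath it.
; The construction script runs the parent's script, then fires a batch of visibility line traces at random points within a small square around the actor.
; Each trace that hits a BP_Tile adds a TreeMeshes instance at the impact location, so trees follow the tile surface and skip other actors.
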(fn `UserConstructionScript`
  (bind _returnvalue (`KismetMathLibrary.RandomPointInBoundingBox` (`self.K2_GetActorLocation`) (`KismetMathLibrary.MakeVector` 100.0 100.0)))
  (`parent.UserConstructionScript`)
  (for _ (range 21)
    (bind (_outhit _returnvalue_2) (`KismetSystemLibrary.LineTraceSingle` (+ _returnvalue (0.0 0.0 100.0)) (+ _returnvalue (0.0 0.0 -100.0)) "TraceTypeQuery1"))
    (if _returnvalue_2
      (bind (_bblockinghit _binitialoverlap _time _location _impactpoint _normal _impactnormal _physmat _hitactor) (`GameplayStatics.BreakHitResult` _outhit))
      (cast `/Game/King/Blueprint/Tiles/BP_Tile` _hitactor)
      (`InstancedStaticMeshComponent.AddInstanceWorldSpace` (`self.TreeMeshes`) (`KismetMathLibrary.Conv_VectorToTransform` _location)))))
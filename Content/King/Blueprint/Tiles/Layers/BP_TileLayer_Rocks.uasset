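; Tile layer Blueprint that scatters rock instances over a tile area.
; After the parent construction script runs, a fixed loop adds world-space instances to the Meshes component at random points in a flat box centered on the actor.
; Each instance gets a random rotation including roll and a random uniform scale, with no seed, so the layout varies whenever construction reruns.
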(fn `UserConstructionScript`
  (`parent.UserConstructionScript`)
  (for _ (range 21)
    (`InstancedStaticMeshComponent.AddInstanceWorldSpace` (`self.Meshes`) (`KismetMathLibrary.MakeTransform` (`KismetMathLibrary.RandomPointInBoundingBox` (`self.K2_GetActorLocation`) (`KismetMathLibrary.MakeVector` 100.0 100.0)) (`KismetMathLibrary.RandomRotator` true) (`KismetMathLibrary.Conv_DoubleToVector` (`KismetMathLibrary.RandomFloatInRange` 0.5 1.5))))))
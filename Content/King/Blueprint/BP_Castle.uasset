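; BP_Castle is a castle Blueprint that creates the ruler and population objects for a kingdom.
; On BeginPlay it constructs a People object, then a King named Alfred Frost with preset starting attributes, storing each in a variable.
; An unconnected chain would construct a Wood Resource and add it to a Resources map, but it never runs.
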(event `self.ReceiveBeginPlay`
  (`|ExecutionSequence`
    (:`then_0`
      (bind _returnvalue (`|GenericCreateObject` "/Game/King/Blueprint/Objects/People.People_C" self))
      (set `self.ThePeople` _returnvalue))
    (:`then_1`
      (bind _returnvalue_2 (`|GenericCreateObject` "/Game/King/Blueprint/Objects/King.King_C" self "Alfred" "Frost" 15.0))
      (set `self.TheKing` _returnvalue_2))))

(fn `UserConstructionScript`)
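; BP_Convoy is a convoy actor that carries a resource payload along tile roads toward a destination.
; It line-traces for the tile beneath it, picks the adjacent road with the fewest steps to the destination, and glides there over a fixed time.
; On arrival it repeats the search, retrying each second on failure.
; Payload unloading to BP_Castle and the return to TownSource exist but are not wired into the running flow.
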(event `Event_TravelToTile`
  (params (Tile :type "/Game/King/Blueprint/Tiles/BP_Tile Object Reference"))
  (`/Engine/EditorBlueprintResources/StandardMacros.IsValid` Tile
    (:`Is Valid`
      (set `self.IsMoving` true)
      (`KismetSystemLibrary.MoveComponentTo` (`self.DefaultSceneRoot`) (`self.K2_GetActorLocation` Tile) (struct) false false 5.0 true)
      (bind _routefound (`self.FindRoute` :!label _label))
      (if (not _routefound)
        (`KismetSystemLibrary.Delay` 1.0)
        (goto _label)))))

(event `self.ReceiveBeginPlay`
  (set `self.StartLocation` (`self.K2_GetActorLocation`))
  (`self.FindRoute`))

(fn `FindRoute`
  (returns (RouteFound :type Boolean))
  (locals (_VisitedRoads :type "Array of /Game/King/Blueprint/Tiles/Layers/BP_TileLayer_Road Object Reference") (_FastestRoute :type "/Game/King/Blueprint/Structs/ST_Route Structure") (_FastestRoad :type "/Game/King/Blueprint/Tiles/Layers/BP_TileLayer_Road Object Reference") (_LowestSteps :type Integer :default 999) (_RouteFound :type Boolean))
  (bind __fastestroad (`local._FastestRoad`))
  (`self.TraceForTile`)
  (`/Engine/EditorBlueprintResources/StandardMacros.IsValid` (`self.TileOn`)
    (:`Is Valid`
      (for _array_element (`/Game/King/Blueprint/Tiles/BP_Tile.AdjacentTiles` (`self.TileOn`))
        (`/Engine/EditorBlueprintResources/StandardMacros.IsValid` _array_element
          (:`Is Valid`
            (bind _road (`/Game/King/Blueprint/Tiles/BP_Tile.GetRoad` _array_element))
            (`/Engine/EditorBlueprintResources/StandardMacros.IsValid` _road
              (:`Is Valid`
                (bind _stepdistance (`/Game/King/Blueprint/Tiles/Layers/BP_TileLayer_Road.GetDistanceToDestination` _road (`self.Destination`)))
                (if (> (`local._LowestSteps`) _stepdistance)
                  (set `local._LowestSteps` _stepdistance)
                  (set `local._FastestRoad` _road)))))))
      (`/Engine/EditorBlueprintResources/StandardMacros.IsValid` __fastestroad
        (:`Is Valid`
          (`self.Event_TravelToTile` (`/Game/King/Blueprint/Tiles/Layers/BP_TileLayer.TileOn` __fastestroad))
          (set `local._RouteFound` true)
          (return (`local._RouteFound`)))))))

(fn `LoadResource`
  (params (ResourceID :type String))
  (`KismetArrayLibrary.Array_Add` (`self.Payload`) ResourceID))

(fn `TraceForTile`
  (bind _returnvalue (`self.K2_GetActorLocation`))
  (bind (_outhit _returnvalue_2) (`KismetSystemLibrary.LineTraceSingle` (+ _returnvalue (0.0 0.0 500.0)) (+ _returnvalue (0.0 0.0 -500.0)) "TraceTypeQuery3"))
  (if _returnvalue_2
    (bind _asbp_tile (cast `/Game/King/Blueprint/Tiles/BP_Tile` (`.HitActor` (`GameplayStatics.BreakHitResult` _outhit))))
    (set `self.TileOn` _asbp_tile)))

(fn `UnloadPayload`
  (bind _payload (`self.Payload`))
  (bind _outactors (`GameplayStatics.GetAllActorsOfClass` "/Game/King/Blueprint/BP_Castle.BP_Castle_C"))
  (for _array_element _outactors :!label _label
    (`/Engine/EditorBlueprintResources/StandardMacros.IsValid` _array_element
      (:`Is Valid`
        (`KismetSystemLibrary.PrintString` (`KismetStringLibrary.Conv_IntToString` (`KismetArrayLibrary.Array_Length` _payload)))
        (for _array_element_2 _payload
          (`/Game/King/Blueprint/BP_Castle.AddResource` _array_element _array_element_2 1)
          (goto _label :!via `Break`))))))

(fn `UserConstructionScript`)
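; Resource object in the King game that tracks a Quantity which can be added to or subtracted from.
; Add and Subtract update Quantity without clamping, then fire the QuantityChanged dispatcher with the resource itself and the amount.
; Both pass Amount unsigned as Diff, so the event alone does not distinguish a gain from a loss.
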(fn `Add`
  (params (Amount :type Integer))
  (set `self.Quantity` (+ Amount (`self.Quantity`)))
  (`self.QuantityChanged` self Amount))

(fn `Subtract`
  (params (Amount :type Integer))
  (set `self.Quantity` (- (`self.Quantity`) Amount))
  (`self.QuantityChanged` self Amount))
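; BP_Builder is a builder actor that moves onto a given tile and drives a build menu through its widget component.
; SetOnTile stores a valid tile, teleports the actor to its location and updates the Widget_BuildMenu with that tile.
; A disconnected line trace that would find a BP_Structure on the tile and show or hide the menu never runs.
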(fn `SetOnTile`
  (params (Tile :type "/Game/King/Blueprint/Tiles/BP_Tile Object Reference"))
  (`/Engine/EditorBlueprintResources/StandardMacros.IsValid` Tile
    (:`Is Valid`
      (bind _output_get (set `self.TileOn` Tile))
      (`self.K2_SetActorLocation` (`self.K2_GetActorLocation` _output_get) false true)
      (bind _aswidget_build_menu (cast `/Game/King/Blueprint/UI/Widgets/Widget_BuildMenu` (`WidgetComponent.GetUserWidgetObject` (`self.Widget`))))
      (`/Game/King/Blueprint/UI/Widgets/Widget_BuildMenu.Update` _aswidget_build_menu (`self.TileOn`)))))

(fn `UserConstructionScript`)
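; Component that registers itself as a stat provider on the tiles around its owner.
; Shortly after BeginPlay, Update resolves a source tile from an owning structure, tile or tile layer, using TileOn for structures and layers.
; It then adds itself to every valid adjacent tile, and to the source tile itself when AddToSource is set.
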(event `self.ReceiveBeginPlay`
  (`KismetSystemLibrary.Delay` 0.2)
  (`self.Update`))

(fn `Update`
  (bind _returnvalue (`self.GetOwner`))
  (bind _sourcetile (`self.SourceTile`))
  (bind _asbp_structure (cast `/Game/King/Blueprint/Structures/BP_Structure` _returnvalue)
    (:`then`
      (bind _tileon (`/Game/King/Blueprint/Structures/BP_Structure.TileOn` _asbp_structure))
      (`/Engine/EditorBlueprintResources/StandardMacros.IsValid` _tileon
        (:`Is Valid`
          (set `self.SourceTile` _tileon))))
    (:`CastFailed`
      (bind _asbp_tile (cast `/Game/King/Blueprint/Tiles/BP_Tile` _returnvalue)
        (:`then`
          (set `self.SourceTile` _asbp_tile))
        (:`CastFailed`
          (bind _asbp_tile_layer (cast `/Game/King/Blueprint/Tiles/Layers/BP_TileLayer` _returnvalue))
          (set `self.SourceTile` (`/Game/King/Blueprint/Tiles/Layers/BP_TileLayer.TileOn` _asbp_tile_layer))))))
  (`/Engine/EditorBlueprintResources/StandardMacros.IsValid` _sourcetile
    (:`Is Valid`
      (`|ExecutionSequence`
        (:`then_0`
          (if (`self.AddToSource`)
            (`/Game/King/Blueprint/Tiles/BP_Tile.AddProvider` (`self.SourceTile`) self)))
        (:`then_1`
          (for _array_element (`/Game/King/Blueprint/Tiles/BP_Tile.AdjacentTiles` _sourcetile)
            (`/Engine/EditorBlueprintResources/StandardMacros.IsValid` _array_element
              (:`Is Valid`
                (`/Game/King/Blueprint/Tiles/BP_Tile.AddProvider` _array_element self)))))))))
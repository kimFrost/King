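; Actor component that periodically produces resources and delivers them to the level's castle.
; On BeginPlay it resets its timer and caches the first BP_Castle found.
; While working, Tick counts down scaled by Efficiency, then adds every BaseProduction output to the castle, shows debug text at the owner and restarts the timer.
; GetTimeLeft exposes the efficiency-adjusted remaining time.
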(event `self.ReceiveBeginPlay`
  (`self.ResetTask`)
  (bind _outactors (`GameplayStatics.GetAllActorsOfClass` "/Game/King/Blueprint/BP_Castle.BP_Castle_C"))
  (for _array_element _outactors
    (set `self.Castle` _array_element)
    (break)))

(event `self.ReceiveTick`
  (params (DeltaSeconds :type "Float (single-precision)"))
  (bind _returnvalue (`self.GetOwner`))
  (bind _castle (`self.Castle`))
  (if (`self.IsWorking`)
    (set `self.TimeLeft` (- (`self.TimeLeft`) (* DeltaSeconds (`self.Efficiency`))))
    (set `self.ScaledTimeLeft` (/ (`self.TimeLeft`) (`self.Efficiency`)))
    (if (<= (`self.TimeLeft`) 0.0)
      (for _array_element (`self.BaseProduction`)
        (bind _output (break `/Game/King/Blueprint/Structs/ST_Production` _array_element))
        (bind _keys (`BlueprintMapLibrary.Map_Keys` _output))
        (for _array_element_2 _keys
          (bind (_value _returnvalue_2) (`BlueprintMapLibrary.Map_Find` _output _array_element_2))
          (if _returnvalue_2
            (`/Engine/EditorBlueprintResources/StandardMacros.IsValid` _castle
              (:`Is Valid`
                (`/Game/King/Blueprint/BP_Castle.AddResource` _castle _array_element_2 _value)
                (`/Engine/EditorBlueprintResources/StandardMacros.IsValid` _returnvalue
                  (:`Is Valid`
                    (`KismetSystemLibrary.DrawDebugString` (`Actor.K2_GetActorLocation` _returnvalue) (`KismetStringLibrary.BuildString_Int` _array_element_2 " x " _value) null (struct :`R` 1.0 :`G` 1.0 :`B` 1.0 :`A` 1.0) 2.0))))))))
      (set `self.TimeLeft` (`self.BaseProductionTime`)))))

(fn `GetTimeLeft`
  (returns (TimeLeft :type "Float (double-precision)"))
  (return (`self.ScaledTimeLeft`)))

(fn `ResetTask`
  (set `self.TimeLeft` (`self.BaseProductionTime`)))
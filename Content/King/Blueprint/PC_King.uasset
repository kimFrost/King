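; Player controller for a hex-tile game that spawns a selector and a builder on BeginPlay and drives both from the mouse cursor.
; Each Tick it traces under the cursor, caches the hit BP_Tile and snaps the Selector to that hex by converting the hit location to cube coordinates and back.
; Right click passes the tile under the cursor to the Builder via SetOnTile.
; Left-click release traces and checks the Builder but performs no action.
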(event `self.ReceiveBeginPlay`
  (bind _returnvalue (`KismetMathLibrary.MakeTransform` (0.0 0.0 0.0)))
  (bind _returnvalue_2 (`|SpawnActorFromClass` "/Game/King/Blueprint/BP_Selector.BP_Selector_C" _returnvalue "AlwaysSpawn" "OverrideRootScale" null null))
  (set `self.Selector` _returnvalue_2)
  (bind _returnvalue_3 (`|SpawnActorFromClass` "/Game/King/Blueprint/BP_Builder.BP_Builder_C" _returnvalue "AlwaysSpawn" "OverrideRootScale" null null))
  (set `self.Builder` _returnvalue_3))

(event `Key|LeftMouseButton`
  (params (Key :type "Key Structure"))
  (:`Released`
    (if (`.ReturnValue` (`self.GetHitResultUnderCursorByChannel` "TraceTypeQuery1"))
      (`/Engine/EditorBlueprintResources/StandardMacros.IsValid` (`self.Builder`)))))

(event `Key|RightMouseButton`
  (params (Key :type "Key Structure")))

(event `self.ReceiveTick`
  (params (DeltaSeconds :type "Float (single-precision)"))
  (bind (_hitresult _returnvalue) (`self.GetHitResultUnderCursorByChannel` "TraceTypeQuery3"))
  (bind _selector (`self.Selector`))
  (bind (_bblockinghit _binitialoverlap _time _location _impactpoint _normal _impactnormal _physmat _hitactor) (`GameplayStatics.BreakHitResult` _hitresult))
  (if _returnvalue
    (bind _asbp_tile (cast `/Game/King/Blueprint/Tiles/BP_Tile` _hitactor)
      (:`then`
        (set `self.TileUnderCursor` _asbp_tile)
        (`/Engine/EditorBlueprintResources/StandardMacros.IsValid` _selector
          (:`Is Valid`
            (bind _returnvalue_2 (`KingTilesLibrary.LocationToCube` 255.0 294.0 _location))
            (bind _returnvalue_3 (`KingTilesLibrary.CubeToLocation` _returnvalue_2))
            (`self.K2_SetActorLocation` _selector _returnvalue_3 false true))))
      (:`CastFailed`
        (set `self.TileUnderCursor` null)))))

(event `Key|RightMouseButton`
  (params (Key :type "Key Structure"))
  (bind (_hitresult _returnvalue) (`self.GetHitResultUnderCursorByChannel` "TraceTypeQuery3" false))
  (bind _builder (`self.Builder`))
  (:`Pressed`
    (if _returnvalue
      (bind _asbp_tile (cast `/Game/King/Blueprint/Tiles/BP_Tile` (`.HitActor` (`GameplayStatics.BreakHitResult` _hitresult))))
      (`/Engine/EditorBlueprintResources/StandardMacros.IsValid` _builder
        (:`Is Valid`
          (`/Game/King/Blueprint/BP_Builder.SetOnTile` _builder _asbp_tile))))))

(fn `UserConstructionScript`)